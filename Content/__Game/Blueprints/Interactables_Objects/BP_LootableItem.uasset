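; BP_LootableItem is an interactable loot container that fills its own inventory with random items and lets the player open it.
; On BeginPlay it initializes its inventory component, then rolls each LootTable entry against a percent chance to add a random quantity.
; Interact passes the player character's inventory and its own to a new WBP_LootInventory widget, then enables the cursor with Game and UI input.
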(event EventInteract
  (params (Player :type Actor%20Object%20Reference))
  (bind _returnvalue (Game|GetPlayerController 0))
  (bind _asbp_third_person_character (Utilities|Casting|CastToBP_ThirdPersonCharacter Player))
  (bind _returnvalue_2 (UserInterface|CreateWidget "/Game/__Game/Widget/Inventory/WBP_LootInventory.WBP_LootInventory_C" (Game|GetPlayerController 0)))
  (Default|InitializeLootInventory _returnvalue_2 (Variables|/Game/__Game/Blueprints/Player/BP_ThirdPersonCharacter.BP_ThirdPersonCharacter_C|GetBP_InventoryComponent _asbp_third_person_character) (Variables|Default|GetBP_InventoryComponent))
  (UserInterface|Viewport|AddtoViewport _returnvalue_2 0)
  (Default|CreateLootSlots _returnvalue_2)
  (Default|RefreshLootInventory _returnvalue_2)
  (Variables|/Script/Engine.PlayerController|SetbShowMouseCursor _returnvalue true)
  (Input|SetInputModeGameandUI _returnvalue 0 "DoNotLock" true false))

(event EventBeginPlay
  (Default|InitializeInventory (Variables|Default|GetBP_InventoryComponent))
  (CallFunction|GenerateLoot))

(fn ConstructionScript)

(fn GenerateLoot
  (for _array_element (Variables|Default|GetLootTable)
    (if (<= (Math|Random|RandomFloatinRange 0.0 1e+02) (.Chance (Utilities|Struct|BreakST_LootEntry _array_element)))
      (Default|AddItem (Variables|Default|GetBP_InventoryComponent) (.ItemDefinition (Utilities|Struct|BreakST_LootEntry _array_element)) (Math|Random|RandomIntegerinRange (.MinQuantity (Utilities|Struct|BreakST_LootEntry _array_element)) (.MaxQuantity (Utilities|Struct|BreakST_LootEntry _array_element)))))))