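; Inventory component that stores item stacks in a fixed number of slots, created empty by InitializeInventory.
; AddItem first checks capacity through CanAddItemInventory, then tops up matching stacks up to MaxStack before spilling the remainder into empty slots.
; SwapItems exchanges two slots by index.
; Crafting-facing functions bridge to the inventory, but only CraftingAddItem is implemented; the can-add, count and remove functions return placeholder values.
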(fn CanAddItemInventory
  (params (ItemDefinition :type PDA%20Item%20Definition%20Object%20Reference) (Quantity :type Integer))
  (Utilities|IsValid ItemDefinition
    (:Is%20Valid
      (LocalVariables|SetMaxStackItemAttempted (Variables|/Game/__Game/Inventory/PDA_ItemDefinition.PDA_ItemDefinition_C|GetMaxStack ItemDefinition))
      (LocalVariables|SetRemaining Quantity)
      (for _array_element (Variables|Default|GetInventory)
        (Utilities|IsValid (.ItemDefinition (Utilities|Struct|BreakST_InventoryItem _array_element))
          (:Is%20Valid
            (if (and (== ItemDefinition (.ItemDefinition (Utilities|Struct|BreakST_InventoryItem _array_element))) (< (.Quantity (Utilities|Struct|BreakST_InventoryItem _array_element)) (Variables|/Game/__Game/Inventory/PDA_ItemDefinition.PDA_ItemDefinition_C|GetMaxStack (.ItemDefinition (Utilities|Struct|BreakST_InventoryItem _array_element)))))
              (bind _output_get (LocalVariables|SetSpaceAvailable (- (Variables|/Game/__Game/Inventory/PDA_ItemDefinition.PDA_ItemDefinition_C|GetMaxStack (.ItemDefinition (Utilities|Struct|BreakST_InventoryItem _array_element))) (.Quantity (Utilities|Struct|BreakST_InventoryItem _array_element)))))
              (LocalVariables|SetNewQuantity (+ (.Quantity (Utilities|Struct|BreakST_InventoryItem _array_element)) (Math|Integer|Min(Integer) (LocalVariables|GetRemaining) _output_get)))
              (LocalVariables|SetRemaining (- (LocalVariables|GetRemaining) (Math|Integer|Min(Integer) (LocalVariables|GetRemaining) _output_get)))))))
      (if (<= (LocalVariables|GetRemaining) 0)
        (return true)
        (else
          (for _array_element_2 (Variables|Default|GetInventory)
            (Utilities|IsValid (.ItemDefinition (Utilities|Struct|BreakST_InventoryItem _array_element_2))
              (:Is%20Not%20Valid
                (LocalVariables|SetRemaining (- (LocalVariables|GetRemaining) (Math|Integer|Min(Integer) (LocalVariables|GetMaxStackItemAttempted) (LocalVariables|GetRemaining)))))))
          (if (<= (LocalVariables|GetRemaining) 0)
            (return true)
            (else
              (return false))))))))

(fn InitializeInventory
  (params (MaxSlots :type Integer))
  (Utilities|Array|Clear (Variables|Default|GetInventory))
  (for _index (range 0 (- MaxSlots 1))
    (Utilities|Array|Add (Variables|Default|GetInventory) (Utilities|Struct|MakeST_InventoryItem))))

(fn AddItem
  (params (ItemDefinition :type PDA%20Item%20Definition%20Object%20Reference) (Quantity :type Integer))
  (bind _maxstack (Variables|/Game/__Game/Inventory/PDA_ItemDefinition.PDA_ItemDefinition_C|GetMaxStack ItemDefinition))
  (LocalVariables|SetRemainingQuantity Quantity)
  (bind _canadd (CallFunction|CanAddItemInventory ItemDefinition (LocalVariables|GetRemainingQuantity)))
  (if _canadd
    (for (_array_element _array_index) (Variables|Default|GetInventory)
      (Utilities|IsValid (.ItemDefinition (Utilities|Struct|BreakST_InventoryItem _array_element))
        (:Is%20Valid
          (LocalVariables|SetCurrent%20Quantity (.Quantity (Utilities|Struct|BreakST_InventoryItem _array_element)))
          (if (== (.ItemDefinition (Utilities|Struct|BreakST_InventoryItem _array_element)) ItemDefinition)
            (if (< (LocalVariables|GetCurrent%20Quantity) (Variables|/Game/__Game/Inventory/PDA_ItemDefinition.PDA_ItemDefinition_C|GetMaxStack (.ItemDefinition (Utilities|Struct|BreakST_InventoryItem _array_element))))
              (LocalVariables|SetAvailable%20Space (- (Variables|/Game/__Game/Inventory/PDA_ItemDefinition.PDA_ItemDefinition_C|GetMaxStack (.ItemDefinition (Utilities|Struct|BreakST_InventoryItem _array_element))) (LocalVariables|GetCurrent%20Quantity)))
              (if (>= (- (Variables|/Game/__Game/Inventory/PDA_ItemDefinition.PDA_ItemDefinition_C|GetMaxStack (.ItemDefinition (Utilities|Struct|BreakST_InventoryItem _array_element))) (LocalVariables|GetCurrent%20Quantity)) (LocalVariables|GetRemainingQuantity))
                (bind _output_get (LocalVariables|SetNew%20Quantity (+ (LocalVariables|GetCurrent%20Quantity) (LocalVariables|GetRemainingQuantity))))
                (Utilities|Array|SetArrayElem (Variables|Default|GetInventory) _array_index (Utilities|Struct|MakeST_InventoryItem (.ItemDefinition (Utilities|Struct|BreakST_InventoryItem _array_element)) _output_get))
                (LocalVariables|SetRemainingQuantity 0)
                (else
                  (Utilities|Array|SetArrayElem (Variables|Default|GetInventory) _array_index (Utilities|Struct|MakeST_InventoryItem ItemDefinition (+ (LocalVariables|GetCurrent%20Quantity) (LocalVariables|GetAvailable%20Space))))
                  (LocalVariables|SetRemainingQuantity (- (LocalVariables|GetRemainingQuantity) (LocalVariables|GetAvailable%20Space))))))))))
    (if (> (LocalVariables|GetRemainingQuantity) 0)
      (for (_array_element_2 _array_index_2) (Variables|Default|GetInventory)
        (Utilities|IsValid (.ItemDefinition (Utilities|Struct|BreakST_InventoryItem _array_element_2))
          (:Is%20Not%20Valid
            (if (> (LocalVariables|GetRemainingQuantity) 0)
              (if (>= _maxstack (LocalVariables|GetRemainingQuantity))
                (Utilities|Array|SetArrayElem (Variables|Default|GetInventory) _array_index_2 (Utilities|Struct|MakeST_InventoryItem ItemDefinition (LocalVariables|GetRemainingQuantity)))
                (LocalVariables|SetRemainingQuantity 0)
                (else
                  (Utilities|Array|SetArrayElem (Variables|Default|GetInventory) _array_index_2 (Utilities|Struct|MakeST_InventoryItem ItemDefinition _maxstack))
                  (LocalVariables|SetRemainingQuantity (- (LocalVariables|GetRemainingQuantity) _maxstack))))))))
      (if (== (LocalVariables|GetRemainingQuantity) 0)
        (return true)
        (else
          (return false)))
      (else
        (return true)))
    (else
      (return false))))

(fn SwapItems
  (params (IndexA :type Integer) (IndexB :type Integer))
  (LocalVariables|SetItemA (Utilities|Array|Get(acopy) (Variables|Default|GetInventory) IndexA))
  (LocalVariables|SetItemB (Utilities|Array|Get(acopy) (Variables|Default|GetInventory) IndexB))
  (Utilities|Array|SetArrayElem (Variables|Default|GetInventory) IndexA (LocalVariables|GetItemB))
  (Utilities|Array|SetArrayElem (Variables|Default|GetInventory) IndexB (LocalVariables|GetItemA)))

(fn CraftingAddItem
  (params (Item :type Item%20Definition%20Base%20Object%20Reference) (Quantity :type Integer))
  (bind _aspda_item_definition (Utilities|Casting|CastToPDA_ItemDefinition Item))
  (bind _success (CallFunction|AddItem _aspda_item_definition Quantity))
  (return _success))

(fn CraftingCanAddItem
  (params (Item :type Item%20Definition%20Base%20Object%20Reference) (Quantity :type Integer))
  (return false))

(fn CraftingGetItemCount
  (params (Item :type Item%20Definition%20Base%20Object%20Reference))
  (return 0))

(fn CraftingRemoveItem
  (params (Item :type Item%20Definition%20Base%20Object%20Reference) (Quantity :type Integer))
  (return false))