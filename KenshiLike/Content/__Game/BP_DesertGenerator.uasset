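; BP_DesertGenerator is a Blueprint that, going by its name, is meant to generate desert layout, though it only computes grid positions so far.
; On BeginPlay, nested loops over GridSizeX and GridSizeY derive X and Y coordinates from Spacing, each offset by a random value within ±RandomJitter.
; The computed positions are not used to spawn or place anything, and the construction script is empty.
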(event EventBeginPlay
  (for _index (range 0 (Variables|Default|GetGridSizeX))
    (for _index_2 (range 0 (Variables|Default|GetGridSizeY))
      (Variables|Default|SetPosX (+ (* _index (Variables|Default|GetSpacing)) (Math|Random|RandomFloatinRange (* (Variables|Default|GetRandomJitter) -1.0) (Variables|Default|GetRandomJitter))))
      (Variables|Default|SetPosY (+ (* _index_2 (Variables|Default|GetSpacing)) (Math|Random|RandomFloatinRange (* (Variables|Default|GetRandomJitter) -1.0) (Variables|Default|GetRandomJitter)))))))

(fn ConstructionScript)