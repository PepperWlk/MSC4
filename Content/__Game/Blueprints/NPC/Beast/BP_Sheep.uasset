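; BP_Sheep is a sheep beast NPC that takes damage and drops loot when killed.
; On any damage it shows the amount on a widget component for a brief delay, then subtracts it from Health.
; At zero health it spawns a lootable item at its location and destroys itself.
; While the damage number is visible, Tick rotates it to face the player camera.
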(event Game|Damage|EventAnyDamage
  (params (Damage :type Float%20%28single-precision%29) (DamageType :type Damage%20Type%20Object%20Reference) (InstigatedBy :type Controller%20Object%20Reference) (DamageCauser :type Actor%20Object%20Reference))
  (bind _damagewidget (Variables|Default|GetDamageWidget))
  (bind _aswbp_damage_number (Utilities|Casting|CastToWBP_DamageNumber (UserInterface|GetUserWidgetObject (Variables|Default|GetDamageWidget))))
  (Default|SetDamage _aswbp_damage_number Damage)
  (Rendering|SetVisibility _damagewidget true false)
  (Utilities|FlowControl|Delay 0.6)
  (Rendering|SetVisibility _damagewidget false false)
  (bind _output_get (Variables|Default|Sethealth (- (Variables|Default|Gethealth) Damage)))
  (if (<= _output_get 0.0)
    (Game|SpawnActorfromClass "/Game/__Game/Blueprints/Interactables_Objects/BP_LootableItem.BP_LootableItem_C" (Math|Transform|MakeTransform (Transformation|GetActorLocation) "0, 0, 0" "1.000000,1.000000,1.000000") "Undefined" "MultiplyWithRoot" 0 0)
    (Actor|DestroyActor)))

(event EventTick
  (params (DeltaSeconds :type Float%20%28single-precision%29))
  (if (Rendering|IsVisible (Variables|Default|GetDamageWidget))
    (Transformation|SetWorldRotation (Variables|Default|GetDamageWidget) (Math|Rotator|FindLookatRotation (Transformation|GetWorldLocation (Variables|Default|GetDamageWidget)) (Camera|GetCameraLocation (Game|GetPlayerCameraManager 0))) false false)))

(fn ConstructionScript)