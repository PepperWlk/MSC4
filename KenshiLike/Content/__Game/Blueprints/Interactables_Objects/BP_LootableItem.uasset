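; BP_LootableItem is an interactable world object that rolls random loot and hands it to the player who interacts with it.
; On BeginPlay it initializes its inventory component and fills it from LootTable, rolling each entry's chance and quantity range independently.
; Interact copies every stack into the character's inventory, clears its own, then destroys the actor after a short delay.
; Debug prints show item names, though GenerateLoot's printed quantity is re-rolled separately from the amount added.
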(event EventInteract
  (params (Player :type Actor%20Object%20Reference))
  (bind _bp_inventorycomponent (Variables|Default|GetBP_InventoryComponent))
  (bind _inventory (Variables|/Game/__Game/Inventory/BP_InventoryComponent.BP_InventoryComponent_C|GetInventory _bp_inventorycomponent))
  (bind _asbp_third_person_character (Utilities|Casting|CastToBP_ThirdPersonCharacter Player))
  (for _array_element _inventory
    (Default|AddItem (Variables|/Game/ThirdPerson/Blueprints/BP_ThirdPersonCharacter.BP_ThirdPersonCharacter_C|GetBP_InventoryComponent _asbp_third_person_character) (.ItemDefinition (Utilities|Struct|BreakST_InventoryItem _array_element)) (.Quantity (Utilities|Struct|BreakST_InventoryItem _array_element)))
    (Development|PrintString (Utilities|GetDisplayName (.ItemDefinition (Utilities|Struct|BreakST_InventoryItem _array_element)))))
  (Utilities|Array|Clear _inventory)
  (Utilities|FlowControl|Delay 0.5)
  (Actor|DestroyActor))

(event EventBeginPlay
  (Default|InitializeInventory (Variables|Default|GetBP_InventoryComponent) 10)
  (CallFunction|GenerateLoot))

(fn ConstructionScript)

(fn GenerateLoot
  (for _array_element (Variables|Default|GetLootTable)
    (if (<= (Math|Random|RandomFloatinRange 0.0 1e+02) (.Chance (Utilities|Struct|BreakST_LootEntry _array_element)))
      (Default|AddItem (Variables|Default|GetBP_InventoryComponent) (.ItemDefinition (Utilities|Struct|BreakST_LootEntry _array_element)) (Math|Random|RandomIntegerinRange (.MinQuantity (Utilities|Struct|BreakST_LootEntry _array_element)) (.MaxQuantity (Utilities|Struct|BreakST_LootEntry _array_element))))
      (Development|PrintString (Utilities|String|Append (Utilities|GetDisplayName (.ItemDefinition (Utilities|Struct|BreakST_LootEntry _array_element))) " : " (Utilities|String|ToString(Integer) (Math|Random|RandomIntegerinRange (.MinQuantity (Utilities|Struct|BreakST_LootEntry _array_element)) (.MaxQuantity (Utilities|Struct|BreakST_LootEntry _array_element)))))))))