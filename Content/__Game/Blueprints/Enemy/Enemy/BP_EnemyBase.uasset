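; BP_EnemyBase is an enemy base Blueprint that handles taking damage and dying.
; AnyDamage passes the damage to a WBP_DamageNumber in DamageWidget and shows it briefly.
; Health is reduced only after that display Delay, so hits landing during it do not each subtract, and the actor is destroyed at zero or below.
; A failed widget cast skips the whole damage response, including the health change.
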(event Game|Damage|EventAnyDamage
  (params (Damage :type Float%20%28single-precision%29) (DamageType :type Damage%20Type%20Object%20Reference) (InstigatedBy :type Controller%20Object%20Reference) (DamageCauser :type Actor%20Object%20Reference))
  (bind _damagewidget (Variables|Default|GetDamageWidget))
  (bind _aswbp_damage_number (Utilities|Casting|CastToWBP_DamageNumber (UserInterface|GetUserWidgetObject (Variables|Default|GetDamageWidget))))
  (Default|SetDamage _aswbp_damage_number Damage)
  (Rendering|SetVisibility _damagewidget true false)
  (Utilities|FlowControl|Delay 0.6)
  (Rendering|SetVisibility _damagewidget false false)
  (bind _output_get (Variables|Default|Sethealth (- (Variables|Default|Gethealth) Damage)))
  (if (<= _output_get 0.0)
    (Actor|DestroyActor)))

(fn ConstructionScript)